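; BP_SpawnPoint is a placed actor that spawns turtles on demand at its own location.
; SpawnTurtle converts an ID to an enum and picks one of three turtle behavior trees from it.
; It spawns a BP_Turtle with that tree, a target point and itself as the spawn point, then plays a summon particle effect and a 2D spawn sound.
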(fn `Spawn Turtle`
  (params (ID :type Integer))
  (bind _returnvalue (`self.K2_GetActorLocation`))
  (switch `/Game/TaskFNTASTIC/Blueprints/EEnumID` (cast `/Game/TaskFNTASTIC/Blueprints/EEnumID` (`KismetMathLibrary.Conv_IntToByte` ID))
    (:`NewEnumerator0`
      (set `self.BehaviorTree` "/Game/TaskFNTASTIC/AI/BehaviorTree/BT_TurtleOne.BT_TurtleOne"))
    (:`NewEnumerator1`
      (set `self.BehaviorTree` "/Game/TaskFNTASTIC/AI/BehaviorTree/BT_TurtleTwo.BT_TurtleTwo"))
    (:`NewEnumerator2`
      (set `self.BehaviorTree` "/Game/TaskFNTASTIC/AI/BehaviorTree/BT_TurtleThree.BT_TurtleThree")))
  (`|SpawnActorFromClass` "/Game/TaskFNTASTIC/AI/Pawn/BP_Turtle.BP_Turtle_C" (`KismetMathLibrary.MakeTransform` _returnvalue) "Undefined" "OverrideRootScale" null (`self.TargetPoint`) (`self.BehaviorTree`) self null)
  (`GameplayStatics.SpawnEmitterAtLocation` "/Game/InfinityBladeEffects/Effects/FX_Ability/Summon/P_Summon_Child_Startup_large.P_Summon_Child_Startup_large" _returnvalue)
  (`GameplayStatics.PlaySound2D` "/Game/TaskFNTASTIC/Sound/MSW_Spawn.MSW_Spawn" 1.0 1.0 0.0 null null))

(fn `UserConstructionScript`)